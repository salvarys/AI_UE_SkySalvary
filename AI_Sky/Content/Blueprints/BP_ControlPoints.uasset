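; BP_ControlPoints is a patrol path that uses the points of a spline as waypoints.
; CircularPatrol advances the patrol index and wraps to the first point, while BouncePatrol steps by a direction value that reverses at either end of the spline.
; GetPointPosition returns the world-space location of the spline point at the current index.
; The index and direction are stored on this Blueprint.
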(event `CircularPatrol`
  (set `self.PatrolIndex` (mod (+ (`self.PatrolIndex`) 1) (`SplineComponent.GetNumberOfSplinePoints` (`self.Spline`)))))

(event `BouncePatrol`
  (bind _output_get (set `self.PatrolIndex` (+ (`self.PatrolIndex`) (`self.direction`))))
  (if (== _output_get (- (`SplineComponent.GetNumberOfSplinePoints` (`self.Spline`)) 1))
    (set `self.direction` -1)
    (elif (== _output_get 0)
      (set `self.direction` 1))))

(fn `GetPointPosition`
  (returns (PointLocation :type "Vector Structure"))
  (return (`SplineComponent.GetLocationAtSplinePoint` (`self.Spline`) (`self.PatrolIndex`) "World")))

(fn `UserConstructionScript`)