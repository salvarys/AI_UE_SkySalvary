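; Actor component that tracks the player's health, starting at the maximum on BeginPlay.
; TakeDamage and Heal adjust current health, clamped between zero and the maximum.
; Every TakeDamage call fires the DamageTaken dispatcher, and reaching zero also fires Dead and prints a debug death message.
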(event `self.ReceiveBeginPlay`
  (set `self.CurrentHealth` (`self.MaxHealth`)))

(fn `Heal`
  (params (HealAmount :type "Float (double-precision)"))
  (set `self.CurrentHealth` (`KismetMathLibrary.FClamp` (+ HealAmount (`self.CurrentHealth`)) 0.0 (`self.MaxHealth`))))

(fn `TakeDamage`
  (params (Damage :type "Float (double-precision)"))
  (bind _output_get (set `self.CurrentHealth` (`KismetMathLibrary.FClamp` (- (`self.CurrentHealth`) Damage) 0.0 (`self.MaxHealth`))))
  (`self.DamageTaken`)
  (if (== _output_get 0.0)
    (`self.Dead`)
    (`KismetSystemLibrary.PrintString` "death, deception, prozaic doom")))