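; BP_Rifle is a rifle pickup that the player equips by walking into its box trigger.
; On BeginPlay it caches the player pawn as BP_ThirdPersonCharacter.
; When that pawn overlaps the Box, it attaches the Rifle component to the character mesh's RifleSocket, snapping location and rotation, and sets HasRifleEquipped on the character.
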(event `self.ReceiveBeginPlay`
  (bind _asbp_third_person_character (cast `/Game/ThirdPerson/Blueprints/BP_ThirdPersonCharacter` (`GameplayStatics.GetPlayerPawn` 0)))
  (set `self.As BP Third Person Character` _asbp_third_person_character))

(event `self.Box.OnComponentBeginOverlap`
  (params (OverlappedComponent :type "PrimitiveComponent Object Reference") (OtherActor :type "Actor Object Reference") (OtherComp :type "PrimitiveComponent Object Reference") (OtherBodyIndex :type Integer) (bFromSweep :type Boolean) (SweepResult :type "HitResult Structure (by ref)"))
  (if (== OtherActor (`GameplayStatics.GetPlayerPawn` 0))
    (`SceneComponent.K2_AttachToComponent` (`self.Rifle`) (`Character.Mesh` (`self.As BP Third Person Character`)) "RifleSocket" "SnapToTarget" "SnapToTarget" "KeepRelative" true)
    (set `/Game/ThirdPerson/Blueprints/BP_ThirdPersonCharacter.HasRifleEquipped` true (`self.As BP Third Person Character`))))

(fn `UserConstructionScript`)